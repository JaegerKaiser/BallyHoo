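; Question card actor that displays one of a fixed set of question faces on its Card mesh.
; The SetQuestion event stores the incoming CardID and switches on it to assign the matching question material to the mesh's first material slot.
; Each question is its own material, covering an original numbered series plus a few newer additions, and the construction script is empty.
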(event `Event SetQuestion`
  (params (CardID :type Integer))
  (bind _card (`self.Card`))
  (bind _output_get (set `self.CardID` CardID))
  (switch `int` _output_get
    (:`0`
      (`PrimitiveComponent.SetMaterial` _card 0 "/Game/Materials/Cards/question_1_Mat.question_1_Mat"))
    (:`1`
      (`PrimitiveComponent.SetMaterial` _card 0 "/Game/Materials/Cards/question_2_Mat.question_2_Mat"))
    (:`2`
      (`PrimitiveComponent.SetMaterial` _card 0 "/Game/Materials/Cards/question_3_Mat.question_3_Mat"))
    (:`3`
      (`PrimitiveComponent.SetMaterial` _card 0 "/Game/Materials/Cards/question_4_Mat.question_4_Mat"))
    (:`4`
      (`PrimitiveComponent.SetMaterial` _card 0 "/Game/Materials/Cards/question_5_Mat.question_5_Mat"))
    (:`5`
      (`PrimitiveComponent.SetMaterial` _card 0 "/Game/Materials/Cards/question_6_Mat.question_6_Mat"))
    (:`6`
      (`PrimitiveComponent.SetMaterial` _card 0 "/Game/Materials/Cards/question_7_Mat.question_7_Mat"))
    (:`7`
      (`PrimitiveComponent.SetMaterial` _card 0 "/Game/Materials/Cards/question_8_Mat.question_8_Mat"))
    (:`8`
      (`PrimitiveComponent.SetMaterial` _card 0 "/Game/Materials/Cards/question_9_Mat.question_9_Mat"))
    (:`9`
      (`PrimitiveComponent.SetMaterial` _card 0 "/Game/Materials/Cards/question_10_Mat.question_10_Mat"))
    (:`10`
      (`PrimitiveComponent.SetMaterial` _card 0 "/Game/Materials/Cards/question_11_Mat.question_11_Mat"))
    (:`11`
      (`PrimitiveComponent.SetMaterial` _card 0 "/Game/Materials/Cards/question_12_Mat.question_12_Mat"))
    (:`12`
      (`PrimitiveComponent.SetMaterial` _card 0 "/Game/Materials/Cards/question_13_Mat.question_13_Mat"))
    (:`13`
      (`PrimitiveComponent.SetMaterial` _card 0 "/Game/Materials/Cards/question_14_Mat.question_14_Mat"))
    (:`14`
      (`PrimitiveComponent.SetMaterial` _card 0 "/Game/Materials/Cards/new_question_1_Mat.new_question_1_Mat"))
    (:`15`
      (`PrimitiveComponent.SetMaterial` _card 0 "/Game/Materials/Cards/new_question_2_Mat.new_question_2_Mat"))
    (:`16`
      (`PrimitiveComponent.SetMaterial` _card 0 "/Game/Materials/Cards/new_question_3_Mat.new_question_3_Mat"))))

(fn `UserConstructionScript`)