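; Question card deck actor that builds and shuffles a fixed set of 18 card IDs and responds to touch.
; InitialiseDeck fills UnshuffledDeck with sequential IDs through CreateDeck.
; ShuffleDeck moves random entries into ShuffledDeck, emptying the source array, then sends the result to LogicBP.
; Touching the actor notifies LogicBP that the deck was pressed.
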(event `InitialiseDeck`
  ;[1 1 1] Create a new deck
  (bind _output_get (set `self.totNumCards` 18))
  (`self.CreateDeck` _output_get))

(event `ShuffleDeck`
  ;[1 1 1] Shuffle
  (bind _shuffleddeck (`self.Shuffle`))
  (set `self.index` 0)
  ;[1 1 1] Send to game logic
  (`/Game/Blueprints/LogicBP.Event SendShuffledQuestionDeck` (`self.LogicBP`) _shuffleddeck))

(event `self.ReceiveActorOnInputTouchBegin`
  (params (FingerIndex :type "ETouchIndex Enum" :default "Touch1"))
  ;[1 1 1] The deck was clicked
  (`/Game/Blueprints/LogicBP.DeckPressed` (`self.LogicBP`)))

(fn `CreateDeck`
  (params (TotalNumberCards :type Integer))
  (bind _cardid (`self.CardID`))
  (bind _unshuffleddeck (`self.unshuffledDeck`))
  ;[1 1 1] Create the deck
  (set `self.CardID` 0)
  (`KismetArrayLibrary.Array_Clear` _unshuffleddeck)
  (`KismetArrayLibrary.Array_Resize` _unshuffleddeck TotalNumberCards)
  (for _index (range TotalNumberCards)
    (`KismetArrayLibrary.Array_Set` _unshuffleddeck _index _cardid)
    (set `self.CardID` (+ _cardid 1)))
  (return))

(fn `Shuffle`
  (returns (ShuffledDeck :type "Array of Integer"))
  (bind _shuffleddeck (`self.shuffledDeck`))
  (bind _shuffleddeck_2 (`self.shuffledDeck`))
  (bind _unshuffleddeck (`self.unshuffledDeck`))
  (bind _random (`self.random`))
  (bind _totnumcards (`self.totNumCards`))
  ;[1 1 1] Shuffle
  (`KismetArrayLibrary.Array_Clear` _shuffleddeck)
  (`KismetArrayLibrary.Array_Resize` _shuffleddeck _totnumcards)
  (for _index (range _totnumcards)
    (set `self.random` (`KismetMathLibrary.RandomIntegerInRange` 0 (`KismetArrayLibrary.Array_LastIndex` (`self.unshuffledDeck`))))
    (`KismetArrayLibrary.Array_Set` _shuffleddeck_2 _index (`|GetArrayItem` _unshuffleddeck _random))
    (`KismetArrayLibrary.Array_Remove` _unshuffleddeck _random))
  (return _shuffleddeck_2))

(fn `UserConstructionScript`)