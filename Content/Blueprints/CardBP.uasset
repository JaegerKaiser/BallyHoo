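; Card Blueprint for a research-methodology card game, each card showing a concept such as a philosophy, methodology or method.
; On construction, CardID is compared against cumulative MaxRed/Yellow/Blue/Green counts to set one of four colour types.
; A switch on CardID, not the type, then applies that concept's material to the Card component.
; SetupCard also calls the material setup, so in-range IDs get it applied twice.
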(fn `SetupCard`
  (params (cardType :type Integer))
  (set `self.currentCardType` cardType)
  (`self.SetupCardMaterial`))

(fn `SetupCardID`
  (params (`Card ID` :type Integer))
  ;[1 1 1] Setting up the card type
  (bind _output_get (set `self.CardID` `Card ID`))
  ;;[1 1 1] Card is Red
  (if (< _output_get (`self.maxRed`))
    (set `self.currentCardType` 0)
    (`self.SetupCard` (`self.currentCardType`) :!label _label)
    (else
      ;;[1 1 1] Card is Yellow
      (if (< _output_get (+ (`self.maxRed`) (`self.maxYellow`)))
        (set `self.currentCardType` 1)
        (goto _label)
        (else
          ;;[1 1 1] Card is Blue
          (if (< _output_get (+ (`self.maxRed`) (`self.maxYellow`) (`self.maxBlue`)))
            (set `self.currentCardType` 2)
            (goto _label)
            (else
              ;;[1 1 1] Card is Green
              (if (< _output_get (+ (`self.maxRed`) (`self.maxYellow`) (`self.maxBlue`) (`self.maxGreen`)))
                (set `self.currentCardType` 3)
                (goto _label)))))))))

(fn `SetupCardMaterial`
  (bind _card (`self.Card`))
  (switch `int` (`self.CardID`)
    (:`0`
      (`PrimitiveComponent.SetMaterial` _card 0 "/Game/Materials/Cards/Constructionism_Mat.Constructionism_Mat"))
    (:`1`
      (`PrimitiveComponent.SetMaterial` _card 0 "/Game/Materials/Cards/Objectivism_Mat.Objectivism_Mat"))
    (:`2`
      (`PrimitiveComponent.SetMaterial` _card 0 "/Game/Materials/Cards/Relativism_Mat.Relativism_Mat"))
    (:`3`
      (`PrimitiveComponent.SetMaterial` _card 0 "/Game/Materials/Cards/Pragmatism_Mat.Pragmatism_Mat"))
    (:`4`
      (`PrimitiveComponent.SetMaterial` _card 0 "/Game/Materials/Cards/Subjectivism_Mat.Subjectivism_Mat"))
    (:`5`
      (`PrimitiveComponent.SetMaterial` _card 0 "/Game/Materials/Cards/Positivism_Mat.Positivism_Mat"))
    (:`6`
      (`PrimitiveComponent.SetMaterial` _card 0 "/Game/Materials/Cards/Interpretivism_-_symbolic_interactionism_Mat.Interpretivism_-_symbolic_interactionism_Mat"))
    (:`7`
      (`PrimitiveComponent.SetMaterial` _card 0 "/Game/Materials/Cards/Interpretivism_-Phenomenology_Mat.Interpretivism_-Phenomenology_Mat"))
    (:`8`
      (`PrimitiveComponent.SetMaterial` _card 0 "/Game/Materials/Cards/Interpretivism_-_Hermeneutics_Mat.Interpretivism_-_Hermeneutics_Mat"))
    (:`9`
      (`PrimitiveComponent.SetMaterial` _card 0 "/Game/Materials/Cards/Ciritical_inquiry_Mat.Ciritical_inquiry_Mat"))
    (:`10`
      (`PrimitiveComponent.SetMaterial` _card 0 "/Game/Materials/Cards/Post_modernism_Mat.Post_modernism_Mat"))
    (:`11`
      (`PrimitiveComponent.SetMaterial` _card 0 "/Game/Materials/Cards/Feminism_Mat.Feminism_Mat"))
    (:`12`
      (`PrimitiveComponent.SetMaterial` _card 0 "/Game/Materials/Cards/Post-positivism_Mat.Post-positivism_Mat"))
    (:`13`
      (`PrimitiveComponent.SetMaterial` _card 0 "/Game/Materials/Cards/Experimental_research_Mat.Experimental_research_Mat"))
    (:`14`
      (`PrimitiveComponent.SetMaterial` _card 0 "/Game/Materials/Cards/Survey_Research_Mat.Survey_Research_Mat"))
    (:`15`
      (`PrimitiveComponent.SetMaterial` _card 0 "/Game/Materials/Cards/Ethnography_Mat.Ethnography_Mat"))
    (:`16`
      (`PrimitiveComponent.SetMaterial` _card 0 "/Game/Materials/Cards/Phenomenological_research_Mat.Phenomenological_research_Mat"))
    (:`17`
      (`PrimitiveComponent.SetMaterial` _card 0 "/Game/Materials/Cards/Grounded_Theory_Mat.Grounded_Theory_Mat"))
    (:`18`
      (`PrimitiveComponent.SetMaterial` _card 0 "/Game/Materials/Cards/Heuristic_inquiry_Mat.Heuristic_inquiry_Mat"))
    (:`19`
      (`PrimitiveComponent.SetMaterial` _card 0 "/Game/Materials/Cards/Action_Research_Mat.Action_Research_Mat"))
    (:`20`
      (`PrimitiveComponent.SetMaterial` _card 0 "/Game/Materials/Cards/Discourse_analysis_Mat.Discourse_analysis_Mat"))
    (:`21`
      (`PrimitiveComponent.SetMaterial` _card 0 "/Game/Materials/Cards/Feminist_standpoint_research_Mat.Feminist_standpoint_research_Mat"))
    (:`22`
      (`PrimitiveComponent.SetMaterial` _card 0 "/Game/Materials/Cards/Sampling_Mat.Sampling_Mat"))
    (:`23`
      (`PrimitiveComponent.SetMaterial` _card 0 "/Game/Materials/Cards/Measurement_and_scaling_Mat.Measurement_and_scaling_Mat"))
    (:`24`
      (`PrimitiveComponent.SetMaterial` _card 0 "/Game/Materials/Cards/Questionnaire_Mat.Questionnaire_Mat"))
    (:`25`
      (`PrimitiveComponent.SetMaterial` _card 0 "/Game/Materials/Cards/Observation_Mat.Observation_Mat"))
    (:`26`
      (`PrimitiveComponent.SetMaterial` _card 0 "/Game/Materials/Cards/Interview_Mat.Interview_Mat"))
    (:`27`
      (`PrimitiveComponent.SetMaterial` _card 0 "/Game/Materials/Cards/Focus_group_Mat.Focus_group_Mat"))
    (:`28`
      (`PrimitiveComponent.SetMaterial` _card 0 "/Game/Materials/Cards/Case_study_Mat.Case_study_Mat"))
    (:`29`
      (`PrimitiveComponent.SetMaterial` _card 0 "/Game/Materials/Cards/Life_history_Mat.Life_history_Mat"))
    (:`30`
      (`PrimitiveComponent.SetMaterial` _card 0 "/Game/Materials/Cards/Narrative_Mat.Narrative_Mat"))
    (:`31`
      (`PrimitiveComponent.SetMaterial` _card 0 "/Game/Materials/Cards/Visual_Ethnography_methods_Mat.Visual_Ethnography_methods_Mat"))
    (:`32`
      (`PrimitiveComponent.SetMaterial` _card 0 "/Game/Materials/Cards/Statistical_Analysis_Mat.Statistical_Analysis_Mat"))
    (:`33`
      (`PrimitiveComponent.SetMaterial` _card 0 "/Game/Materials/Cards/Data_reduction_Mat.Data_reduction_Mat"))
    (:`34`
      (`PrimitiveComponent.SetMaterial` _card 0 "/Game/Materials/Cards/theme_identification_Mat.theme_identification_Mat"))
    (:`35`
      (`PrimitiveComponent.SetMaterial` _card 0 "/Game/Materials/Cards/Comparative_analysis_Mat.Comparative_analysis_Mat"))
    (:`36`
      (`PrimitiveComponent.SetMaterial` _card 0 "/Game/Materials/Cards/Cognitive_mapping_Mat.Cognitive_mapping_Mat"))
    (:`37`
      (`PrimitiveComponent.SetMaterial` _card 0 "/Game/Materials/Cards/Interpretative_methods_Mat.Interpretative_methods_Mat"))
    (:`38`
      (`PrimitiveComponent.SetMaterial` _card 0 "/Game/Materials/Cards/Document_analysis_Mat.Document_analysis_Mat"))
    (:`39`
      (`PrimitiveComponent.SetMaterial` _card 0 "/Game/Materials/Cards/Content_analysis_Mat.Content_analysis_Mat"))
    (:`40`
      (`PrimitiveComponent.SetMaterial` _card 0 "/Game/Materials/Cards/Conversation_analysis_Mat.Conversation_analysis_Mat"))))

(fn `UserConstructionScript`
  ;[1 1 1] Setup card colour and material on spawn
  (`self.SetupCardID` (`self.CardID`))
  (`self.SetupCardMaterial`))